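; Openable door actor that swings around its yaw axis when it receives open and close events.
; It records its starting rotation and location at BeginPlay.
; The OpenDoor timeline plays on open and reverses on close, adding its angle track to the starting rotation.
; An event track on the timeline times the door lock sound, played at the starting location.
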(event OnOpen(OpenDoor)
  (bind _open_angle (Timeline|Open%20Door Play)
    (:Update
      (Transformation|SetActorRotation (Math|Rotator|CombineRotators (Variables|Default|GetInitialRotation) (Math|Rotator|MakeRotator 0.0 0.0 _open_angle))))
    (:SoundTiming
      (Audio|PlaySoundatLocation "/Game/Audio/door-lock.door-lock" (Variables|Default|GetInitalLocation)))))

(event OnClose(OpenDoor)
  (bind _open_angle (Timeline|Open%20Door Reverse)
    (:Update
      (Transformation|SetActorRotation (Math|Rotator|CombineRotators (Variables|Default|GetInitialRotation) (Math|Rotator|MakeRotator 0.0 0.0 _open_angle))))
    (:SoundTiming
      (Audio|PlaySoundatLocation "/Game/Audio/door-lock.door-lock" (Variables|Default|GetInitalLocation)))))

(event EventBeginPlay
  (Variables|Default|SetInitialRotation (Transformation|GetActorRotation))
  (Variables|Default|SetInitalLocation (Transformation|GetActorLocation)))

(fn ConstructionScript)